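; Player character that moves along one axis and carries the temple's HP, resources and construction state.
; GainHP builds temple stages at HP thresholds, escalates spawner waves and triggers victory, with tutorial variants that jump construction straight to the final stage.
; AnyDamage lowers HP, destroys stages after an earthquake faked by alternating LaunchCharacter impulses, and pauses on game over at zero.
; The resource-check popup timer and pause-menu nodes are unwired.
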(event `InputAxis|move right`
  (params (AxisValue :type "Float (single-precision)"))
  (bind _returnvalue (`self.GetTransform`))
  ;[1 1 1] Mouvement droite gauche caméra
  (`self.K2_SetActorTransform` (`KismetMathLibrary.MakeTransform` (+ (`KismetMathLibrary.TransformDirection` _returnvalue (`KismetMathLibrary.MakeVector` (* (* AxisValue (`self.SpeedMove`)) 1.0))) (.location _returnvalue)))))

(event `InputAction|TestA`
  (params (Key :type "Key Structure"))
  ;[1 0 0] Zone test  DEV ONLY
)

(event `self.ReceiveAnyDamage`
  (params (Damage :type "Float (single-precision)") (DamageType :type "DamageType Object Reference") (InstigatedBy :type "Controller Object Reference") (DamageCauser :type "Actor Object Reference"))
  (bind _hp (`self.HP`))
  ;[1 1 1] Système perte PV / mort / ÉVENEMENT QUAND ON PERD DE LA VIE
  (set `self.HP` (- (`self.HP`) Damage))
  (if (and (< _hp 450.0) (and (`self.Stage2Constructed`) (`self.Stage3Construct`)))
    (`/Engine/EditorBlueprintResources/StandardMacros.DoOnce` false :!label _label
      (:`Completed`
        (`self.Earthquake`)
        (`KismetSystemLibrary.Delay` 4.0)
        (set `self.Stage3Construct` false)
        (`self.K2_DestroyActor` (`self.stage3`))
        (goto _label :!via `Reset`)))
    (elif (and (< _hp 150.0) (`self.Stage2Constructed`))
      (`/Engine/EditorBlueprintResources/StandardMacros.DoOnce` false :!label _label_2
        (:`Completed`
          (`self.Earthquake`)
          (`KismetSystemLibrary.Delay` 4.0)
          (set `self.Stage2Constructed` false)
          (`self.K2_DestroyActor` (`self.stage2`))
          (goto _label_2 :!via `Reset`)))
      (elif (< (`self.HP`) 1.0)
        (`GameplayStatics.SetGamePaused` true)
        (if (`self.IsInLevelTuto`)
          (bind _returnvalue (`|CreateWidget` "/Game/HUD/WB_GameOverTuto.WB_GameOverTuto_C"))
          (`UserWidget.AddToViewport` _returnvalue 0)
          (`GameplayStatics.PlaySound2D` "/Game/Sources/SoundDesign/Events/GameOverSound.GameOverSound" 1.0 1.0 0.0 null null)
          (else
            (bind _returnvalue_2 (`|CreateWidget` "/Game/HUD/WB_GameOver.WB_GameOver_C"))
            (`UserWidget.AddToViewport` _returnvalue_2 0)
            (`GameplayStatics.PlaySound2D` null 1.0 1.0 0.0 null null)))))))

(event `InputAction|TestB`
  (params (Key :type "Key Structure"))
  ;[1 0 0] Zone test  DEV ONLY
)

(event `Earthquake`
  ;[1 1 1] Tremblement de terre
  (`GameplayStatics.PlaySound2D` "/Game/Sources/SoundDesign/Earthquake/Eathquake_cue.Eathquake_cue" 3.0 1.0 0.0 null null)
  (set `self.EndEarthquake` false)
  (`|ExecutionSequence`
    (:`then_0`
      (if (not (`self.EndEarthquake`)) :!label _label_3
        (`self.LaunchCharacter` (0.0 0.0 300.0))
        (`KismetSystemLibrary.Delay` 0.05)
        (`self.LaunchCharacter` (0.0 0.0 -20000.0))
        (`KismetSystemLibrary.Delay` 0.05)
        (goto _label_3)))
    (:`then_1`
      (`KismetSystemLibrary.Delay` 4.0)
      (set `self.EndEarthquake` true)
      (`GameplayStatics.PlaySound2D` "/Game/Sources/SoundDesign/Eboulement/Eboulement_wav.Eboulement_wav" 0.7 1.0 1.2 null null))
    (:`then_2`
      (bind _returnvalue (`GameplayStatics.GetActorOfClass` "/Game/Elements/SpawnPoint.SpawnPoint_C"))
      (set `self.SpawnPointRef` _returnvalue))))

(event `self.ReceiveBeginPlay`
  (`|ExecutionSequence`
    (:`then_0`
      (bind _returnvalue (`GameplayStatics.GetActorOfClass` "/Game/Elements/SpawnPoint.SpawnPoint_C"))
      (set `self.SpawnPointRef` _returnvalue)
      (bind _returnvalue_2 (`GameplayStatics.GetActorOfClass` "/Game/Elements/SpawnBoss.SpawnBoss_C"))
      (set `self.SpawnBossRef` _returnvalue_2)
      (bind _returnvalue_3 (`GameplayStatics.GetActorOfClass` "/Game/Elements/SpawnPointTuto.SpawnPointTuto_C"))
      (set `self.SpawnTutoRef` _returnvalue_3)
      (bind _returnvalue_4 (`GameplayStatics.GetActorOfClass` "/Game/Elements/SpawnBossTuto.SpawnBossTuto_C"))
      (set `self.SpawnBossTutoRef` _returnvalue_4))
    (:`then_1`
      (bind _returnvalue_5 (`GameplayStatics.GetActorOfClass` "/Game/Elements/TestBizare/BoostEnnemies.BoostEnnemies_C"))
      (set `self.BoostRef` _returnvalue_5))))

(event `WidgetTemple`
  (if (and (and (>= (`self.Brick`) 60) (>= (`self.Iron`) 60)) (and (>= (`self.Wood`) 60) (>= (`self.Glass`) 60)))
    (`/Engine/EditorBlueprintResources/StandardMacros.DoOnce` false
      (:`Completed`
        (bind _returnvalue (`|CreateWidget` "/Game/Dialogues/Onboarding_Tower/WB_TempleTuto.WB_TempleTuto_C"))
        (`UserWidget.AddToViewport` _returnvalue 0)))))

(fn `ConstructStage`
  (if (`self.IsInLevelTuto`)
    (set `self.Stage2Constructed` true)
    (set `self.Stage3Construct` true)
    (`|SpawnActorFromClass` "/Game/MainCharacter/StagesOfTemples/BP_Stage4.BP_Stage4_C" (`KismetMathLibrary.MakeTransform` (`self.SpawnStageLocation`)) "Undefined" "OverrideRootScale" null null)
    (`GameplayStatics.PlaySound2D` "/Game/Sources/SoundDesign/Temple/TempleConstructMetal.TempleConstructMetal" 0.9 1.0 0.0 null null)
    (`GameplayStatics.PlaySound2D` "/Game/Sources/SoundDesign/Temple/TempleConstructWood.TempleConstructWood" 0.9 1.0 0.0 null null)
    (bind _returnvalue (`|CreateWidget` "/Game/Dialogues/WB_DialoguesEnding.WB_DialoguesEnding_C"))
    (`UserWidget.AddToViewport` _returnvalue 0)
    (`GameplayStatics.SetGamePaused` true)
    (set `self.HP` 1000.0)
    (return)
    (elif (== (`self.StageRef`) "/Game/MainCharacter/StagesOfTemples/BP_Stage2.BP_Stage2_C")
      (bind _returnvalue_2 (`|SpawnActorFromClass` "/Game/MainCharacter/StagesOfTemples/BP_Stage2.BP_Stage2_C" (`KismetMathLibrary.MakeTransform` (`self.SpawnStageLocation`)) "Undefined" "OverrideRootScale" null null))
      (`GameplayStatics.PlaySound2D` "/Game/Sources/SoundDesign/Temple/TempleConstructMetal.TempleConstructMetal" 0.9 1.0 0.0 null null)
      (`GameplayStatics.PlaySound2D` "/Game/Sources/SoundDesign/Temple/TempleConstructWood.TempleConstructWood" 0.9 1.0 0.0 null null)
      (set `self.stage2` _returnvalue_2)
      (return)
      (elif (== (`self.StageRef`) "/Game/MainCharacter/StagesOfTemples/BP_Stage3.BP_Stage3_C")
        (bind _returnvalue_3 (`|SpawnActorFromClass` "/Game/MainCharacter/StagesOfTemples/BP_Stage3.BP_Stage3_C" (`KismetMathLibrary.MakeTransform` (`self.SpawnStageLocation`)) "Undefined" "OverrideRootScale" null null))
        (`GameplayStatics.PlaySound2D` "/Game/Sources/SoundDesign/Temple/TempleConstructMetal.TempleConstructMetal" 0.9 1.0 0.0 null null)
        (`GameplayStatics.PlaySound2D` "/Game/Sources/SoundDesign/Temple/TempleConstructWood.TempleConstructWood" 0.9 1.0 0.0 null null)
        (set `self.stage3` _returnvalue_3)
        (return)
        (else
          (`|SpawnActorFromClass` "/Game/MainCharacter/StagesOfTemples/BP_Stage4.BP_Stage4_C" (`KismetMathLibrary.MakeTransform` (`self.SpawnStageLocation`)) "Undefined" "OverrideRootScale" null null)
          (`GameplayStatics.PlaySound2D` "/Game/Sources/SoundDesign/Temple/TempleConstructMetal.TempleConstructMetal" 0.9 1.0 0.0 null null)
          (`GameplayStatics.PlaySound2D` "/Game/Sources/SoundDesign/Temple/TempleConstructWood.TempleConstructWood" 0.9 1.0 0.0 null null))))))

(fn `GainHP`
  (params (HPgived :type "Float (double-precision)"))
  (bind _hp (`self.HP`))
  (bind _spawntutoref (`self.SpawnTutoRef`))
  (bind _spawnbossref (`self.SpawnBossRef`))
  (bind _spawntutoref_2 (`self.SpawnTutoRef`))
  (bind _spawnbosstutoref (`self.SpawnBossTutoRef`))
  (bind _boostref (`self.BoostRef`))
  (bind _spawnpointref (`self.SpawnPointRef`))
  (bind _spawnpointref_2 (`self.SpawnPointRef`))
  (bind _spawnbossref_2 (`self.SpawnBossRef`))
  (bind _spawnbossref_3 (`self.SpawnBossRef`))
  ;[1 1 1] Regagner des PV sans passer par les événement de perte de PV / ÉVENEMENTS DE GAINS DE PV
  (set `self.HP` (+ HPgived _hp))
  (if (>= _hp 1000.0)
    ;;[1 0.5368 0.4869] Etage 4
    (set `self.YouCanConstruct` true)
    (`self.SetStageLocation` (10600.0 3300.0 300.0))
    (set `self.StageRef` "/Game/MainCharacter/StagesOfTemples/BP_Stage4.BP_Stage4_C")
    (`self.ConstructStage`)
    (`GameplayStatics.SetGamePaused` true)
    (`GameplayStatics.PlaySound2D` "/Game/Sources/SoundDesign/Events/VictorySound.VictorySound" 1.0 1.0 0.0 null null)
    (if (`self.IsInLevelTuto`)
      (bind _returnvalue (`|CreateWidget` "/Game/Dialogues/WB_DialoguesEnding.WB_DialoguesEnding_C"))
      (`UserWidget.AddToViewport` _returnvalue 0)
      (else
        (`GameplayStatics.SetGamePaused` true)
        (`GameplayStatics.PlaySound2D` null 1.0 1.0 0.0 null null)
        (bind _returnvalue_2 (`|CreateWidget` "/Game/HUD/WB_Win.WB_Win_C"))
        (`UserWidget.AddToViewport` _returnvalue_2 0)))
    (return)
    (elif (>= _hp 600.0)
      (set `self.YouCanConstruct` true)
      (set `self.Stage3Construct` true)
      (set `self.StageRef` "/Game/MainCharacter/StagesOfTemples/BP_Stage3.BP_Stage3_C")
      (`self.SetStageLocation` (10600.0 3300.0 200.0))
      (`self.ConstructStage`)
      (if (`self.IsInLevelTuto`)
        (`/Game/Elements/SpawnPointTuto.Set Spawn Wave 3` _spawntutoref false)
        (`/Game/Elements/SpawnPointTuto.Set Speed Spawn` _spawntutoref 2.9)
        (`/Game/Elements/SpawnPointTuto.Set Spawn Wave 3` _spawntutoref true)
        (`/Game/Elements/SpawnPointTuto.Wave3` _spawntutoref)
        (`/Game/Elements/SpawnBoss.SetSpawnWave2` _spawnbossref false)
        (`/Game/Elements/SpawnBoss.StartingWave3` _spawnbossref)
        (else
          (`/Game/Elements/TestBizare/BoostEnnemies.SetWave2Boost` _boostref false)
          (`/Game/Elements/TestBizare/BoostEnnemies.SetWave3Boost` _boostref true)
          (`/Game/Elements/SpawnPoint.SetSpawnWave2` _spawnpointref false)
          (`/Game/Elements/SpawnPoint.Set Speed Spawn` _spawnpointref 3.0)
          (`/Game/Elements/SpawnPoint.Set Spawn Wave 3` _spawnpointref true)
          (`/Game/Elements/SpawnPoint.Wave 3` _spawnpointref)
          (`/Game/Elements/SpawnBoss.SetSpawnWave2` _spawnbossref_2 false)
          (`/Game/Elements/SpawnBoss.StartingWave3` _spawnbossref_2)))
      (return)
      (else
        (if (`self.Stage3Construct`)
          _
          (else
            _))
        (if (and (>= _hp 300.0) (not (`self.Stage2Constructed`)))
          (set `self.YouCanConstruct` true)
          (set `self.Stage2Constructed` true)
          (set `self.StageRef` "/Game/MainCharacter/StagesOfTemples/BP_Stage2.BP_Stage2_C")
          (`self.SetStageLocation` (10600.0 3300.0 180.0))
          (`self.ConstructStage`)
          (if (`self.IsInLevelTuto`)
            (`/Game/Elements/SpawnPointTuto.set Starting spawn B` _spawntutoref_2 false)
            (`/Game/Elements/SpawnPointTuto.Set Speed Spawn` _spawntutoref_2 3.7)
            (`/Game/Elements/SpawnPointTuto.SetSpawnWave2` _spawntutoref_2 true)
            (`/Game/Elements/SpawnPointTuto.Wave2` _spawntutoref_2)
            (`/Game/Elements/SpawnBossTuto.Set Spawn Wave 1` _spawnbosstutoref false)
            (`/Game/Elements/SpawnBossTuto.StartingWave2` _spawnbosstutoref)
            (else
              (`/Game/Elements/TestBizare/BoostEnnemies.SetWave2Boost` (`self.BoostRef`) true)
              (`/Game/Elements/SpawnPoint.set Starting spawn B` _spawnpointref_2 false)
              (`/Game/Elements/SpawnPoint.Set Speed Spawn` _spawnpointref_2 3.2)
              (`/Game/Elements/SpawnPoint.SetSpawnWave2` _spawnpointref_2 true)
              (`/Game/Elements/SpawnPoint.Wave2` _spawnpointref_2)
              (`/Game/Elements/SpawnBoss.Set Spawn Wave 1` _spawnbossref_3 false)
              (`/Game/Elements/SpawnBoss.StartingWave2` _spawnbossref_3)))
          (return)
          (elif (`self.Stage2Constructed`)
            _))))))

(fn `SetBrick`
  (params (Brick :type Integer))
  (set `self.Brick` Brick)
  (return))

(fn `SetGlass`
  (params (Glass :type Integer))
  (set `self.Glass` Glass)
  (return))

(fn `SetHP`
  (params (HP :type "Float (double-precision)"))
  (set `self.HP` HP)
  (return))

(fn `SetIron`
  (params (Iron :type Integer))
  (set `self.Iron` Iron)
  (return))

(fn `SetMoney`
  (params (Money :type Integer))
  (set `self.Money` Money)
  (return))

(fn `SetStageLocation`
  (params (SpawnStageLocation :type "Vector Structure"))
  (set `self.SpawnStageLocation` SpawnStageLocation)
  (return))

(fn `SetWood`
  (params (Wood :type Integer))
  (set `self.Wood` Wood)
  (return))

(fn `UserConstructionScript`)