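; Parent Blueprint for a turret slot: a clickable area that toggles a WB_TurretSelect widget component for choosing a turret.
; AreaTurret swaps materials on hover, release and click; opening the menu first calls AffichageWidget on all WB_TurretSelect widgets.
; BeginPlay cross-links slot and widget, while small functions set spawn location and spawned state or reset the widget's spawned flag.
; Two unconnected test chains never run.
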(event `self.AreaTurret.OnBeginCursorOver`
  (params (TouchedComponent :type "PrimitiveComponent Object Reference"))
  ;[1 1 1] Begin Cursor Over
  (`PrimitiveComponent.SetMaterial` (`self.AreaTurret`) 0 "/Game/LevelPrototyping/Materials/MI_Solid_Blue.MI_Solid_Blue"))

(event `self.AreaTurret.OnEndCursorOver`
  (params (TouchedComponent :type "PrimitiveComponent Object Reference"))
  ;[1 1 1] End Cursor Over
  (`PrimitiveComponent.SetMaterial` (`self.AreaTurret`) 0 "/Game/Sources/Assets/Slot/M_Slot.M_Slot"))

(event `self.AreaTurret.OnReleased`
  (params (TouchedComponent :type "PrimitiveComponent Object Reference") (ButtonReleased :type "Key Structure"))
  ;[1 1 1] Released
  (`PrimitiveComponent.SetMaterial` (`self.AreaTurret`) 0 "/Game/StarterContent/Materials/M_AssetPlatform.M_AssetPlatform"))

(event `self.AreaTurret.OnClicked`
  (params (TouchedComponent :type "PrimitiveComponent Object Reference") (ButtonPressed :type "Key Structure"))
  (bind _areaturret (`self.AreaTurret`))
  (bind _wb_turretselect (`self.WB_TurretSelect`))
  (if (`SceneComponent.IsVisible` (`self.WB_TurretSelect`))
    ;[1 1 1] Visibility si widget
    (`PrimitiveComponent.SetMaterial` _areaturret 0 "/Game/StarterContent/Materials/M_Metal_Gold.M_Metal_Gold")
    (`SceneComponent.SetVisibility` _wb_turretselect false false)
    (else
      ;[1 1 1] Visibility si pas de widget
      (bind _foundwidgets (`WidgetBlueprintLibrary.GetAllWidgetsOfClass` "/Game/HUD/WB_TurretSelect.WB_TurretSelect_C" false))
      (for _index (range (+ (`KismetArrayLibrary.Array_Length` _foundwidgets) 1))
        (bind _output (`|GetArrayItem` _foundwidgets _index))
        (`/Engine/EditorBlueprintResources/StandardMacros.IsValid` _output
          (:`Is Valid`
            (`/Game/HUD/WB_TurretSelect.AffichageWidget` _output))))
      (`PrimitiveComponent.SetMaterial` _areaturret 0 "/Game/enemies/Skeletal_Meshes/M_Brick.M_Brick")
      (`SceneComponent.SetVisibility` _wb_turretselect true false))))

(event `self.ReceiveBeginPlay`
  (bind _aswb_turret_select (cast `/Game/HUD/WB_TurretSelect` (`WidgetComponent.GetUserWidgetObject` (`self.WB_TurretSelect`))))
  (set `/Game/HUD/WB_TurretSelect.TurretSlotRef` self _aswb_turret_select)
  (set `self.TurretSelectRef` _aswb_turret_select))

(fn `SetButtons`
  (bind _aswb_turret_select (cast `/Game/HUD/WB_TurretSelect` (`WidgetComponent.GetWidget` (`self.WB_TurretSelect`))))
  (`/Game/HUD/WB_TurretSelect.SetTurretSpawned` _aswb_turret_select false)
  (return))

(fn `SetTurretSpawned`
  (params (TurretSpawned :type Boolean))
  (set `self.TurretSpawned` TurretSpawned)
  (return))

(fn `setTurretSpawnLoc`
  (params (TurretSpawnLocation :type "Vector Structure"))
  (returns (spawn :type "Vector Structure"))
  (bind _output_get (set `self.TurretSpawnLocation` TurretSpawnLocation))
  (return _output_get))

(fn `UserConstructionScript`)