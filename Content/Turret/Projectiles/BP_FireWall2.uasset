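; BP_FireWall2 is a short-lived fire wall from the turret projectiles that knocks back and burns enemies, destroying itself after a fixed delay.
; RepulsiveBox overlap launches BP_EnemiesParent characters along a fixed world X axis, regardless of the wall's rotation.
; HitBox overlap copies the wall's burning damage, speed and time onto the enemy, then calls its Burning function.
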(event `self.ReceiveBeginPlay`
  (`KismetSystemLibrary.Delay` 3.0)
  (`self.K2_DestroyActor`))

(event `self.RepulsiveBox.OnComponentBeginOverlap`
  (params (OverlappedComponent :type "PrimitiveComponent Object Reference") (OtherActor :type "Actor Object Reference") (OtherComp :type "PrimitiveComponent Object Reference") (OtherBodyIndex :type Integer) (bFromSweep :type Boolean) (SweepResult :type "HitResult Structure (by ref)"))
  (bind _asbp_enemies_parent (cast `/Game/enemies/BP_EnemiesParent` OtherActor))
  (`Character.LaunchCharacter` _asbp_enemies_parent (10000.0 0.0 0.0) false false))

(event `self.HitBox.OnComponentBeginOverlap`
  (params (OverlappedComponent :type "PrimitiveComponent Object Reference") (OtherActor :type "Actor Object Reference") (OtherComp :type "PrimitiveComponent Object Reference") (OtherBodyIndex :type Integer) (bFromSweep :type Boolean) (SweepResult :type "HitResult Structure (by ref)"))
  (bind _asbp_enemies_parent (cast `/Game/enemies/BP_EnemiesParent` OtherActor))
  (`/Game/enemies/BP_EnemiesParent.SetBurningdamage` _asbp_enemies_parent (`self.Burning Damage`))
  (`/Game/enemies/BP_EnemiesParent.SetBurningSpeed` _asbp_enemies_parent (`self.Burning Speed`))
  (`/Game/enemies/BP_EnemiesParent.SetBurningTime` _asbp_enemies_parent (`self.Burning Time`))
  (`/Game/enemies/BP_EnemiesParent.Burning` _asbp_enemies_parent))

(fn `UserConstructionScript`)