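; Turret projectile that poisons enemies it touches.
; On BulletCollision overlap, it casts the other actor to BP_EnemiesParent, copies its poison time, speed and damage onto that enemy, then calls the enemy's Poison function.
; The projectile only supplies the parameters, leaving the effect itself to the enemy; its event graph holds no movement or destruction logic.
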(event `self.BulletCollision.OnComponentBeginOverlap`
  (params (OverlappedComponent :type "PrimitiveComponent Object Reference") (OtherActor :type "Actor Object Reference") (OtherComp :type "PrimitiveComponent Object Reference") (OtherBodyIndex :type Integer) (bFromSweep :type Boolean) (SweepResult :type "HitResult Structure (by ref)"))
  (bind _asbp_enemies_parent (cast `/Game/enemies/BP_EnemiesParent` OtherActor))
  (`/Game/enemies/BP_EnemiesParent.setpoisonTime` _asbp_enemies_parent (`self.Poison Time`))
  (`/Game/enemies/BP_EnemiesParent.SetPoisonSpeed` _asbp_enemies_parent (`self.Poisonspeed`))
  (`/Game/enemies/BP_EnemiesParent.SetPoisondamage` _asbp_enemies_parent (`self.Poison Damage`))
  (`/Game/enemies/BP_EnemiesParent.Poison` _asbp_enemies_parent))

(fn `UserConstructionScript`
  (`parent.UserConstructionScript`))