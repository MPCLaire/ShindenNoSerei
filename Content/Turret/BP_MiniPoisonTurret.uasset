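; Mini poison turret that targets BP_TurretParent actors entering its detection volume, picking one at random and firing projectiles at it.
; Gated, self-calling Delay loops turn Base yaw and clamped Depression pitch toward the target, or rotate back toward zero when none remains.
; The aim loop also drives delayed shots from OutOfCannon, adding direct damage when IsSniper is set.
; Incoming damage depletes HP until the turret bursts in a particle effect and is destroyed.
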(event `SelectTarget`
  (bind _targetinrange (`self.TargetInRange`))
  ;[1 1 1] Select Target
  (if (`KismetArrayLibrary.Array_IsValidIndex` _targetinrange)
    ;;[1 0 0.1081] target
    (set `self.Target` (`|GetArrayItem` _targetinrange (`KismetMathLibrary.RandomIntegerInRange` 0 (`KismetArrayLibrary.Array_LastIndex` _targetinrange))))
    (`self.BeginAim`)
    (else
      (`self.BeginReset`))))

(event `self.OverlapDetection.OnComponentBeginOverlap`
  (params (OverlappedComponent :type "PrimitiveComponent Object Reference") (OtherActor :type "Actor Object Reference") (OtherComp :type "PrimitiveComponent Object Reference") (OtherBodyIndex :type Integer) (bFromSweep :type Boolean) (SweepResult :type "HitResult Structure (by ref)"))
  ;[1 1 1] Ciblage
  (bind _asbp_turret_parent (cast `/Game/Turret/BP_TurretParent` OtherActor))
  (`KismetArrayLibrary.Array_Add` (`self.TargetInRange`) _asbp_turret_parent)
  (`self.SelectTarget`))

(event `self.OverlapDetection.OnComponentEndOverlap`
  (params (OverlappedComponent :type "PrimitiveComponent Object Reference") (OtherActor :type "Actor Object Reference") (OtherComp :type "PrimitiveComponent Object Reference") (OtherBodyIndex :type Integer))
  (bind _targetinrange (`self.TargetInRange`))
  ;[1 1 1] Ciblage
  (bind _asbp_turret_parent (cast `/Game/Turret/BP_TurretParent` OtherActor))
  (if (`KismetArrayLibrary.Array_Contains` _targetinrange _asbp_turret_parent)
    (`KismetArrayLibrary.Array_RemoveItem` _targetinrange _asbp_turret_parent)
    (if (== _asbp_turret_parent (`self.Target`))
      ;;[1 0 0.06238] target
      (set `self.Target` null)
      (`self.SelectTarget`))))

(event `ContinueReset`
  (bind _returnvalue (`GameplayStatics.GetWorldDeltaSeconds`))
  (bind _returnvalue_2 (`KismetMathLibrary.RInterpTo_Constant` (`SceneComponent.RelativeRotation` (`self.Base`)) (struct) _returnvalue 50.0))
  (bind _returnvalue_3 (`KismetMathLibrary.RInterpTo_Constant` (`SceneComponent.RelativeRotation` (`self.Base`)) (struct) _returnvalue 50.0))
  ;[1 1 1] Système de Reset
  (`/Engine/EditorBlueprintResources/StandardMacros.Gate` true :!label _label
    (:`Exit`
      (`/Engine/EditorBlueprintResources/StandardMacros.IsValid` (`self.Target`)
        (:`Is Valid`
          (`self.CancelReset` :!label _label_2))
        (:`Is Not Valid`
          (if (and (== _returnvalue_3 (struct)) (== _returnvalue_2 (struct)))
            (goto _label_2)
            (else
              (`SceneComponent.K2_SetRelativeRotation` (`self.Base`) _returnvalue_3 false false)
              (`SceneComponent.K2_SetRelativeRotation` (`self.Depression`) _returnvalue_2 false false)
              (`KismetSystemLibrary.Delay` _returnvalue)
              (`self.ContinueReset`))))))))

(event `BeginReset`
  ;[1 1 1] Système de Reset
  (`|ExecutionSequence`
    (:`then_0`
      (goto _label :!via `Open`))
    (:`then_1`
      (goto _label))))

(event `CancelReset`
  ;[1 1 1] Système de Reset
  (goto _label :!via `Close`))

(event `ContinueAim`
  (bind _returnvalue (`GameplayStatics.GetWorldDeltaSeconds`))
  (bind _target (`self.Target`))
  (bind _speedrot (`self.SpeedRot`))
  (bind (_returnvalue_roll _returnvalue_pitch _returnvalue_yaw) (`KismetMathLibrary.BreakRotator` (`KismetMathLibrary.MakeRotFromX` (`KismetMathLibrary.InverseTransformDirection` (`self.GetTransform`) (- (`SceneComponent.K2_GetComponentLocation` (`self.Depression`)) (`self.TargetLocation`))))))
  ;[1 1 1] Aim
  ;;[1 0 0.1472] taret
  (`/Engine/EditorBlueprintResources/StandardMacros.IsValid` (`self.Target`)
    (:`Is Valid`
      ;;[1 1 1] IA des tourelles
      (`/Engine/EditorBlueprintResources/StandardMacros.Gate` true :!label _label_3
        (:`Exit`
          (`/Engine/EditorBlueprintResources/StandardMacros.IsValid` (`self.Target`)
            (:`Is Valid`
              ;;[1 1 1] Get Target Location
              (set `self.TargetLocation` (+ (`self.K2_GetActorLocation` _target) (* (`self.GetVelocity` _target) 0.0)))
              (`|ExecutionSequence`
                (:`then_0`
                  (`SceneComponent.K2_SetRelativeRotation` (`self.Base`) (`KismetMathLibrary.RInterpTo_Constant` (`SceneComponent.RelativeRotation` (`self.Base`)) (`KismetMathLibrary.MakeRotator` 0.0 0.0 _returnvalue_yaw) _returnvalue _speedrot) false false)
                  (`SceneComponent.K2_SetRelativeRotation` (`self.Depression`) (`KismetMathLibrary.MakeRotator` (.roll (`KismetMathLibrary.RInterpTo_Constant` (`SceneComponent.RelativeRotation` (`self.Depression`)) (`KismetMathLibrary.MakeRotator` 0.0 _returnvalue_pitch) _returnvalue _speedrot)) (`KismetMathLibrary.ClampAngle` (.pitch (`KismetMathLibrary.RInterpTo_Constant` (`SceneComponent.RelativeRotation` (`self.Depression`)) (`KismetMathLibrary.MakeRotator` 0.0 _returnvalue_pitch) _returnvalue _speedrot)) (`self.MinAngleDepression`) (`self.MaxAngleDepression`)) (.yaw (`KismetMathLibrary.RInterpTo_Constant` (`SceneComponent.RelativeRotation` (`self.Depression`)) (`KismetMathLibrary.MakeRotator` 0.0 _returnvalue_pitch) _returnvalue _speedrot))) false false)
                  (`KismetSystemLibrary.Delay` _returnvalue)
                  (`self.ContinueAim`))
                (:`then_1`
                  ;;[0.6375 0.1159 0.1007] Tir (Appel de la fonction Shot)
                  (`KismetSystemLibrary.Delay` (`self.FireRate`))
                  (`self.Shot` self (`self.ProjectileVariable`))
                  (if (`self.IsSniper`)
                    (`GameplayStatics.ApplyDamage` (`self.Target`) (`self.DamageSniper`))))))
            (:`Is Not Valid`
              (`self.CancelAim` :!label _label_4)
              (`self.BeginReset`))))))
    (:`Is Not Valid`
      (goto _label_4))))

(event `BeginAim`
  ;[1 1 1] Aim
  (`|ExecutionSequence`
    (:`then_0`
      (goto _label_3 :!via `Open`))
    (:`then_1`
      (goto _label_3))))

(event `CancelAim`
  ;[1 1 1] Aim
  (goto _label_3 :!via `Close`))

(event `self.ReceiveAnyDamage`
  (params (Damage :type "Float (single-precision)") (DamageType :type "DamageType Object Reference") (InstigatedBy :type "Controller Object Reference") (DamageCauser :type "Actor Object Reference"))
  (bind _hp (`self.HP`))
  (set `self.HP` (- _hp Damage))
  (if (<= _hp 0.0)
    (`GameplayStatics.SpawnEmitterAtLocation` "/Game/FXVarietyPack/Particles/P_ky_waterBallHit.P_ky_waterBallHit" (`self.K2_GetActorLocation`) (struct) (8.0 8.0 8.0))
    (`self.K2_DestroyActor`)))

(event `self.ReceiveBeginPlay`
  (bind _aswb_turret_select (cast `/Game/HUD/WB_TurretSelect` (`WidgetComponent.GetUserWidgetObject` (`self.Turretselect`))))
  (set `self.TurretSelectRef` _aswb_turret_select))

(fn `Shot`
  (params (TypeOfProjectile :type "Actor Class Reference"))
  (`|SpawnActorFromClass` TypeOfProjectile (`SceneComponent.K2_GetComponentToWorld` (`self.OutOfCannon`)) "Undefined" "OverrideRootScale" null null))

(fn `UserConstructionScript`)