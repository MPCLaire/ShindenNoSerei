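; BP_MiniPoisonTurret2 is a destructible turret that, despite its name, spawns BP_FireRateBoost actors while facing other turrets in its range.
; Box overlaps maintain a list of BP_TurretParent actors within the area.
; A repeating Delay loop picks a random turret from that list, snaps to face it and spawns the boost at the Sphere's transform.
; Incoming damage lowers HP and destroys the actor at zero.
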(event `self.ReceiveBeginPlay`
  (`self.Waiting`))

(event `SelectTarget`
  (bind _turretref (`self.TurretRef`))
  (if (`KismetArrayLibrary.Array_IsValidIndex` _turretref)
    (set `self.target` (`|GetArrayItem` _turretref (`KismetMathLibrary.RandomIntegerInRange` 0 (`KismetArrayLibrary.Array_LastIndex` _turretref))))
    (`self.Attack`)
    (else
      (`self.Waiting`))))

(event `Attack`
  (`self.K2_SetActorRotation` (`KismetMathLibrary.FindLookAtRotation` (`self.K2_GetActorLocation`) (`self.K2_GetActorLocation` (`self.target`))))
  (`|SpawnActorFromClass` "/Game/Turret/Projectiles/BP_FireRateBoost.BP_FireRateBoost_C" (`SceneComponent.K2_GetComponentToWorld` (`self.Sphere`)) "Undefined" "OverrideRootScale" null null)
  (`self.Waiting`))

(event `Waiting`
  (`KismetSystemLibrary.Delay` 7.0)
  (`self.SelectTarget`))

(event `self.Box.OnComponentBeginOverlap`
  (params (OverlappedComponent :type "PrimitiveComponent Object Reference") (OtherActor :type "Actor Object Reference") (OtherComp :type "PrimitiveComponent Object Reference") (OtherBodyIndex :type Integer) (bFromSweep :type Boolean) (SweepResult :type "HitResult Structure (by ref)"))
  (bind _asbp_turret_parent (cast `/Game/Turret/BP_TurretParent` OtherActor))
  (`KismetArrayLibrary.Array_Add` (`self.TurretRef`) _asbp_turret_parent))

(event `self.Box.OnComponentEndOverlap`
  (params (OverlappedComponent :type "PrimitiveComponent Object Reference") (OtherActor :type "Actor Object Reference") (OtherComp :type "PrimitiveComponent Object Reference") (OtherBodyIndex :type Integer))
  (bind _turretref (`self.TurretRef`))
  (bind _asbp_turret_parent (cast `/Game/Turret/BP_TurretParent` OtherActor))
  (if (`KismetArrayLibrary.Array_Contains` _turretref _asbp_turret_parent)
    (`KismetArrayLibrary.Array_RemoveItem` _turretref _asbp_turret_parent)))

(event `self.ReceiveAnyDamage`
  (params (Damage :type "Float (single-precision)") (DamageType :type "DamageType Object Reference") (InstigatedBy :type "Controller Object Reference") (DamageCauser :type "Actor Object Reference"))
  (bind _hp (`self.HP`))
  (set `self.HP` (- _hp Damage))
  (if (<= _hp 0.0)
    (`self.K2_DestroyActor`)))

(fn `UserConstructionScript`)