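; Base enemy character that walks to the GoalOfEnemis actor, retrying on failure, then destroys itself and damages the player.
; Incoming damage updates a floating health bar, and death plays a sound and pays money and resources to the player.
; Vacuum, Burning and Poison events run timed delay loops for repeated launches or self-damage, tuned through setters alongside speed and health bonuses.
; Mesh sway logic is present but unconnected.
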(event `self.ReceiveTick`
  (params (DeltaSeconds :type "Float (single-precision)"))
  ;[1 1 1] Code mvt ennemis
)

(event `self.ReceiveBeginPlay`
  (bind _returnvalue (`GameplayStatics.GetActorOfClass` "/Game/MainCharacter/BP_MainCharacter2.BP_MainCharacter2_C"))
  (set `self.MainCharacterRef` _returnvalue)
  (`self.GoToGoal`)
  (bind _asfloating_bar (cast `/Game/HUD/FloatingBar` (`WidgetComponent.GetUserWidgetObject` (`self.HPbar`))))
  (set `self.HealthWidgetRef` _asfloating_bar)
  (set `/Game/HUD/FloatingBar.HealthMax` (`self.HPmax`) _asfloating_bar)
  (set `/Game/HUD/FloatingBar.Health` (`self.HP`) _asfloating_bar)
  (`Widget.SetVisibility` _asfloating_bar "Hidden"))

(event `GoToGoal`
  ;[1 1 1] Go to goal
  (`KismetSystemLibrary.Delay` 0.2)
  (set `CharacterMovementComponent.MaxWalkSpeed` (`self.speedMove`) (`self.CharacterMovement`))
  (bind _outactors (`GameplayStatics.GetAllActorsOfClass` "/Game/Elements/GoalOfEnemis.GoalOfEnemis_C"))
  (`|AIMoveTo` self (0.0 0.0 0.0) (`|GetArrayItem` _outactors) 200.0
    (:`OnSuccess`
      (`self.K2_DestroyActor`)
      (`GameplayStatics.ApplyDamage` (`self.MainCharacterRef`) (`self.Degat`)))
    (:`OnFail`
      (`self.GoToGoal`))))

(event `self.ReceiveAnyDamage`
  (params (Damage :type "Float (single-precision)") (DamageType :type "DamageType Object Reference") (InstigatedBy :type "Controller Object Reference") (DamageCauser :type "Actor Object Reference"))
  (bind _hp (`self.HP`))
  (bind _healthwidgetref (`self.HealthWidgetRef`))
  (bind _maincharacterref (`self.MainCharacterRef`))
  ;[1 1 1] Damages
  (bind _output_get (set `self.HP` (- _hp Damage)))
  (set `/Game/HUD/FloatingBar.Health` _output_get _healthwidgetref)
  (`Widget.SetVisibility` _healthwidgetref "Visible")
  (if (<= _hp 0.0)
    (`self.K2_DestroyActor`)
    (`GameplayStatics.PlaySound2D` "/Game/Sources/SoundDesign/Enemies/RandomSoundsEnemiesDying.RandomSoundsEnemiesDying" 0.25 0.9 0.0 null null)
    ;[1 1 1] Ressources
    (`/Game/MainCharacter/BP_MainCharacter2.SetMoney` _maincharacterref (+ (`/Game/MainCharacter/BP_MainCharacter2.Money` _maincharacterref) (`self.MoneyLoot`)))
    (`/Game/MainCharacter/BP_MainCharacter2.SetIron` _maincharacterref (+ (`self.IronLoot`) (`/Game/MainCharacter/BP_MainCharacter2.Iron` _maincharacterref)))
    (`/Game/MainCharacter/BP_MainCharacter2.SetWood` _maincharacterref (+ (`self.woodLoot`) (`/Game/MainCharacter/BP_MainCharacter2.Wood` _maincharacterref)))
    (`/Game/MainCharacter/BP_MainCharacter2.SetBrick` _maincharacterref (+ (`self.brickLoot`) (`/Game/MainCharacter/BP_MainCharacter2.Brick` _maincharacterref)))
    (`/Game/MainCharacter/BP_MainCharacter2.SetGlass` _maincharacterref (+ (`self.GlassLoot`) (`/Game/MainCharacter/BP_MainCharacter2.Glass` _maincharacterref)))))

(event `Vacuum`
  (bind _charactermovement (`self.CharacterMovement`))
  ;[1 1 1] aspiration
  (set `self.Aspiration` false)
  (`|ExecutionSequence`
    (:`then_0`
      (set `CharacterMovementComponent.MaxWalkSpeed` 0.0 _charactermovement)
      (if (not (`self.Aspiration`)) :!label _label
        (`self.LaunchCharacter` (`self.Launch Velocity`))
        (`KismetSystemLibrary.Delay` 0.05)
        (`self.LaunchCharacter` (`self.Launch Velocity`))
        (`KismetSystemLibrary.Delay` 0.05)
        (goto _label)))
    (:`then_1`
      (`KismetSystemLibrary.Delay` 3.0)
      (set `self.Aspiration` true)
      (set `CharacterMovementComponent.MaxWalkSpeed` (`self.speedMove`) _charactermovement))))

(event `Burning`
  ;[1 1 1] Burning (tourelle AoE)
  (set `self.Cooking` true)
  (`|ExecutionSequence`
    (:`then_0`
      (if (`self.Cooking`) :!label _label_2
        (`GameplayStatics.ApplyDamage` self (`self.BurningDamage`))
        (`KismetSystemLibrary.Delay` (`self.BurningSpeed`))
        (`GameplayStatics.ApplyDamage` self (`self.BurningDamage`))
        (`KismetSystemLibrary.Delay` 0.25)
        (goto _label_2)))
    (:`then_1`
      (`KismetSystemLibrary.Delay` (`self.BurningTime`))
      (set `self.Cooking` false))))

(event `Poison`
  ;[1 1 1] Poison
  (set `self.Poisoning` true)
  (`|ExecutionSequence`
    (:`then_0`
      (if (`self.Poisoning`) :!label _label_3
        (`GameplayStatics.ApplyDamage` self (`self.PoisonDamage`))
        (`KismetSystemLibrary.Delay` (`self.Poisonspeed`))
        (`GameplayStatics.ApplyDamage` self (`self.PoisonDamage`))
        (`KismetSystemLibrary.Delay` 0.2)
        (goto _label_3)))
    (:`then_1`
      (`KismetSystemLibrary.Delay` (`self.PoisonTime`))
      (set `self.Poisoning` false))))

(fn `SetAspiration`
  (params (`Launch Velocity` :type "Vector Structure"))
  (set `self.Launch Velocity` `Launch Velocity`)
  (return))

(fn `SetBurningdamage`
  (params (BurningDamage :type "Float (single-precision)"))
  (set `self.BurningDamage` BurningDamage)
  (return))

(fn `SetBurningSpeed`
  (params (BurningSpeed :type "Float (single-precision)"))
  (set `self.BurningSpeed` BurningSpeed)
  (return))

(fn `SetBurningTime`
  (params (BurningTime :type "Float (single-precision)"))
  (set `self.BurningTime` BurningTime)
  (return))

(fn `SetHealth`
  (params (HPbonus :type "Float (double-precision)"))
  (bind _output_get (set `self.HP` (+ HPbonus (`self.HP`))))
  (set `self.HPmax` _output_get)
  (return))

(fn `SetPoisondamage`
  (params (PoisonDamage :type "Float (single-precision)"))
  (set `self.PoisonDamage` PoisonDamage)
  (return))

(fn `SetPoisonSpeed`
  (params (Poisonspeed :type "Float (single-precision)"))
  (set `self.Poisonspeed` Poisonspeed)
  (return))

(fn `setpoisonTime`
  (params (PoisonTime :type "Float (single-precision)"))
  (set `self.PoisonTime` PoisonTime)
  (return))

(fn `SetSpeed`
  (params (speedMoveBonus :type "Float (double-precision)"))
  (set `self.speedMove` (+ (`self.speedMove`) speedMoveBonus))
  (return))

(fn `UserConstructionScript`)