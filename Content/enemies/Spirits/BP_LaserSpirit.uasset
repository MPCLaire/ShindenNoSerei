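; BP_LaserSpirit is an enemy spirit that wanders and fires lasers at turrets.
; It moves to random reachable points via AI MoveTo, then picks a random turret tracked by its detection box overlaps, or moves again if none.
; It faces the target once, loops charge particles until a timed ready flag flips, then spawns BP_Laser.
; After firing it resumes wandering, or destroys itself in the tutorial level.
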(event `self.ReceiveBeginPlay`
  (`parent.ReceiveBeginPlay`)
  (`KismetSystemLibrary.Delay` 5.0)
  (`self.Patern`)
  (bind _returnvalue (`GameplayStatics.GetActorOfClass` "/Game/MainCharacter/BP_MainCharacter2.BP_MainCharacter2_C"))
  (set `self.MaincharacterRef` _returnvalue))

(event `select target`
  (bind _turretsref (`self.TurretsRef`))
  ;[1 1 1] selectioner une cible
  (if (`KismetArrayLibrary.Array_IsValidIndex` _turretsref)
    (set `self.TargetSelected` (`|GetArrayItem` _turretsref (`KismetMathLibrary.RandomIntegerInRange` 0 (`KismetArrayLibrary.Array_LastIndex` _turretsref))))
    (`self.Attack`)
    (else
      (`self.Patern`))))

(event `Attack`
  (bind _sphere (`self.Sphere`))
  (bind _returnvalue (`SceneComponent.K2_GetComponentLocation` _sphere))
  ;[1 0.6354 0.6354] Viser
  (`self.K2_SetActorRotation` (`KismetMathLibrary.FindLookAtRotation` (`self.K2_GetActorLocation`) (`self.K2_GetActorLocation` (`self.TargetSelected`))))
  (`|ExecutionSequence`
    (:`then_0`
      ;[1 0.3424 0.3822] Chargement du tir
      (if (`self.ReadyToShoot`) :!label _label
        ;[1 0 0.04978] Tir + renvois au mouvement random
        (`GameplayStatics.SpawnEmitterAtLocation` "/Game/StarterContent/Particles/P_Explosion.P_Explosion" _returnvalue (struct) (3.0 3.0 3.0))
        (`|SpawnActorFromClass` "/Game/enemies/Spirits/SpiritsAttacks/BP_Laser.BP_Laser_C" (`SceneComponent.K2_GetComponentToWorld` _sphere) "Undefined" "OverrideRootScale" null null)
        (`GameplayStatics.PlaySound2D` "/Game/Sources/SoundDesign/Spirits/MiniBossTurretSound.MiniBossTurretSound" 0.3 1.0 0.0 null null)
        (if (`/Game/MainCharacter/BP_MainCharacter2.IsInLevelTuto` (`self.MaincharacterRef`))
          (`KismetSystemLibrary.Delay` 2.0)
          (`self.K2_DestroyActor`)
          (else
            (`KismetSystemLibrary.Delay` 2.0)
            (`self.Patern`)
            (set `self.ReadyToShoot` false)))
        (else
          (`GameplayStatics.SpawnEmitterAtLocation` "/Game/FXVarietyPack/Particles/P_ky_hit1.P_ky_hit1" _returnvalue)
          (`KismetSystemLibrary.Delay` 0.2)
          (`GameplayStatics.SpawnEmitterAtLocation` "/Game/FXVarietyPack/Particles/P_ky_hit1.P_ky_hit1" _returnvalue)
          (`KismetSystemLibrary.Delay` 0.2)
          (goto _label))))
    (:`then_1`
      (`KismetSystemLibrary.Delay` 10.0)
      (set `self.ReadyToShoot` true))))

(event `Patern`
  ;[0.2809 1 0.3832] mouvement random
  (`|AIMoveTo` self (`NavigationSystemV1.K2_GetRandomReachablePointInRadius` (`self.K2_GetActorLocation`) 500.0 null null) null
    (:`OnSuccess`
      (`self.select target`))
    (:`OnFail`
      (`self.Patern`))))

(event `self.DetectionBox.OnComponentBeginOverlap`
  (params (OverlappedComponent :type "PrimitiveComponent Object Reference") (OtherActor :type "Actor Object Reference") (OtherComp :type "PrimitiveComponent Object Reference") (OtherBodyIndex :type Integer) (bFromSweep :type Boolean) (SweepResult :type "HitResult Structure (by ref)"))
  ;[1 0.8565 0.05967] Ajouter une cible
  (bind _asbp_turret_parent (cast `/Game/Turret/BP_TurretParent` OtherActor))
  (`KismetArrayLibrary.Array_Add` (`self.TurretsRef`) _asbp_turret_parent))

(event `self.DetectionBox.OnComponentEndOverlap`
  (params (OverlappedComponent :type "PrimitiveComponent Object Reference") (OtherActor :type "Actor Object Reference") (OtherComp :type "PrimitiveComponent Object Reference") (OtherBodyIndex :type Integer))
  (bind _turretsref (`self.TurretsRef`))
  ;[1 0.8565 0.05967] Ajouter une cible
  (bind _asbp_turret_parent (cast `/Game/Turret/BP_TurretParent` OtherActor))
  (if (`KismetArrayLibrary.Array_Contains` _turretsref _asbp_turret_parent)
    (`KismetArrayLibrary.Array_RemoveItem` _turretsref _asbp_turret_parent)))

(fn `UserConstructionScript`
  (`parent.UserConstructionScript`))