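; Spirit enemy that wanders the level and spawns BP_Portal actors, commented as enemy teleportation portals.
; After BeginPlay, a self-repeating Patern event moves it to random reachable points, dropping a portal on each arrival.
; A DetectionBox tracks nearby enemies for SelectTarget, which nothing here calls.
; That branch moves to a random tracked enemy and spawns a portal with sound, then resumes wandering or self-destructs in the tutorial.
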(event `self.ReceiveBeginPlay`
  (`parent.ReceiveBeginPlay`)
  (`KismetSystemLibrary.Delay` 5.0)
  (`self.Patern`)
  (bind _returnvalue (`GameplayStatics.GetActorOfClass` "/Game/MainCharacter/BP_MainCharacter2.BP_MainCharacter2_C"))
  (set `self.MainCharacterRef` _returnvalue))

(event `GoToTarget`
  ;[1 1 1] Aller vers la cible sélectioner
  (`|AIMoveTo` self (`self.K2_GetActorLocation` (`self.TargetSelected`)) null
    (:`OnSuccess`
      (`self.SpawnPortal`))
    (:`OnFail`
      (`self.Patern`))))

(event `SpawnPortal`
  ;[1 1 1] Faire spawn portail de téléportation des ennemis
  (`|SpawnActorFromClass` "/Game/enemies/Spirits/SpiritsAttacks/BP_Portal.BP_Portal_C" (`self.GetTransform`) "Undefined" "OverrideRootScale" null null)
  (`GameplayStatics.PlaySound2D` "/Game/Sources/SoundDesign/Spirits/MiniBossPortalSound.MiniBossPortalSound" 0.5 1.0 0.0 null null)
  (if (`/Game/MainCharacter/BP_MainCharacter2.IsInLevelTuto` (`self.MaincharacterRef`))
    (`KismetSystemLibrary.Delay` 2.0)
    (`self.K2_DestroyActor`)
    (else
      (`KismetSystemLibrary.Delay` 1.5)
      (`self.Patern`))))

(event `Patern`
  ;[1 1 1] Mouvement Random
  (`KismetSystemLibrary.Delay` 3.0)
  (`|AIMoveTo` self (`NavigationSystemV1.K2_GetRandomReachablePointInRadius` (`self.K2_GetActorLocation`) 2500.0 null null) null
    (:`OnSuccess`
      (`|SpawnActorFromClass` "/Game/enemies/Spirits/SpiritsAttacks/BP_Portal.BP_Portal_C" (`self.GetTransform`) "Undefined" "OverrideRootScale" null null)
      (`self.Patern`))
    (:`OnFail`
      (`self.Patern`))))

(event `SelectTarget`
  (bind _ennemisref (`self.EnnemisRef`))
  ;[1 1 1] Choisir une cible aléatoire
  (if (`KismetArrayLibrary.Array_IsValidIndex` _ennemisref)
    (set `self.TargetSelected` (`|GetArrayItem` _ennemisref (`KismetMathLibrary.RandomIntegerInRange` 0 (`KismetArrayLibrary.Array_LastIndex` _ennemisref))))
    (`self.GoToTarget`)
    (else
      (`self.Patern`))))

(event `self.DetectionBox.OnComponentBeginOverlap`
  (params (OverlappedComponent :type "PrimitiveComponent Object Reference") (OtherActor :type "Actor Object Reference") (OtherComp :type "PrimitiveComponent Object Reference") (OtherBodyIndex :type Integer) (bFromSweep :type Boolean) (SweepResult :type "HitResult Structure (by ref)"))
  ;[1 1 1] Ajouter une cible / désajouter
  (bind _asbp_enemies_parent (cast `/Game/enemies/BP_EnemiesParent` OtherActor))
  (`KismetArrayLibrary.Array_Add` (`self.EnnemisRef`) _asbp_enemies_parent))

(event `self.DetectionBox.OnComponentEndOverlap`
  (params (OverlappedComponent :type "PrimitiveComponent Object Reference") (OtherActor :type "Actor Object Reference") (OtherComp :type "PrimitiveComponent Object Reference") (OtherBodyIndex :type Integer))
  (bind _ennemisref (`self.EnnemisRef`))
  ;[1 1 1] Ajouter une cible / désajouter
  (bind _asbp_enemies_parent (cast `/Game/enemies/BP_EnemiesParent` OtherActor))
  (if (`KismetArrayLibrary.Array_Contains` _ennemisref _asbp_enemies_parent)
    (`KismetArrayLibrary.Array_RemoveItem` _ennemisref _asbp_enemies_parent)))

(fn `UserConstructionScript`
  (`parent.UserConstructionScript`))